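; Enemy character that scans for the player while standing still and passes a spotted player to its AI.
; Each tick at zero velocity it enables scanning and interpolates a Yaw value between positive and negative limits; moving disables scanning and zeroes Yaw.
; A static mesh overlap during scanning writes a player-controlled BP_Character to the blackboard's TargetActor key.
; A red debug line is drawn every tick along the head socket's forward direction.
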(event OnComponentBeginOverlap(StaticMesh)
  (params (OverlappedComponent :type Primitive%20Component%20Object%20Reference) (OtherActor :type Actor%20Object%20Reference) (OtherComp :type Primitive%20Component%20Object%20Reference) (OtherBodyIndex :type Integer) (bFromSweep :type Boolean) (SweepResult :type Hit%20Result%20Structure%20%28by%20ref%29))
  (if (Variables|Default|GetScanning)
    (bind _asbp_character (Utilities|Casting|CastToBP_Character OtherActor))
    (Utilities|Casting|CastToPlayerController (Pawn|GetController _asbp_character))
    (AI|Components|Blackboard|SetValueasObject (Variables|/Script/AIModule.AIController|GetBlackboard (AI|GetAIController self)) (Utilities|Name|MakeLiteralName "TargetActor") _asbp_character)))

(event Custom|SetScanning
  (params (Scanning :type Boolean))
  (Variables|Default|SetScanning Scanning)
  (if Scanning
    _))

(event EventTick
  (params (DeltaSeconds :type Float%20%28single-precision%29))
  (bind _mesh (Variables|Character|GetMesh))
  (bind _returnvalue (Transformation|GetSocketTransform _mesh "headSocket" "RTS_World"))
  (Utilities|FlowControl|Sequence
    (:then_0
      (if (== (Math|Vector|VectorLength (Transformation|GetVelocity)) 0.0)
        (CallFunction|SetScanning true)
        (bind _output_get (Variables|Default|SetYaw (Math|Interpolation|FInterpTo (Variables|Default|GetYaw) (* (Variables|Default|GetDirection) (Variables|Default|GetMaxRotation)) DeltaSeconds (Variables|Default|GetInterpSpeed))))
        (if (Math|Float|NearlyEqual(Float) _output_get (* (Variables|Default|GetMaxRotation) (Variables|Default|GetDirection)) 1.0)
          (Variables|Default|SetDirection (* (Variables|Default|GetDirection) -1.0)))
        (else
          (CallFunction|SetScanning false)
          (Variables|Default|SetYaw 0.0))))
    (:then_1
      (Rendering|Debug|DrawDebugLine (.location _returnvalue) (+ (.location _returnvalue) (* (Math|Vector|GetForwardVector (.rotation _returnvalue)) 8e+02)) "(R=1.000000,G=0.000000,B=0.042499,A=1.000000)" 0.0 1e+01))))

(fn ConstructionScript)