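; Game mode that handles player spawning, checkpoint respawns and level-change notifications.
; BeginPlay seeds the saved teleport destination from the first PlayerSpawnPoint found and spawns the player.
; Respawn spawns and possesses a new BP_Character above that destination, then destroys all DestructibleActors; OnPlayerDeath increments Tries before respawning.
; Destination updates and the level one/two events call OnLevelChanged, which is empty here.
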(event Custom|OnLevelChanged
  (params (LevelNum :type Integer)))

(event Custom|OnLevelOne
  (CallFunction|OnLevelChanged 1))

(event Custom|OnLEvelTwo
  (CallFunction|OnLevelChanged 2))

(event EventBeginPlay
  (bind _outactors (Actor|GetAllActorsOfClass "/Game/KrakJam/PlayerSpawnPoint.PlayerSpawnPoint_C"))
  (CallFunction|SetLastTeleportDestination (Transformation|GetActorLocation (Utilities|Array|Get(acopy) _outactors)) (Transformation|GetActorRotation (Utilities|Array|Get(acopy) _outactors)))
  (CallFunction|Respawn))

(event EventTick
  (params (DeltaSeconds :type Float%20%28single-precision%29)))

(fn ConstructionScript)

(fn OnPlayerDeath
  (Math|Integer|IncrementInt (Variables|Default|GetTries)
    (:%20%20
      (CallFunction|Respawn))))

(fn SetLastTeleportDestination
  (params (Location :type Vector) (Rotation :type Rotator) (LevelNum :type Integer))
  (Variables|Default|SetLastTeleportDestination Location)
  (Variables|Default|SetLastTeleportRotation Rotation)
  (bind _output_get (Variables|Default|SetLevelNum LevelNum))
  (CallFunction|OnLevelChanged _output_get))

(fn Respawn
  (bind _returnvalue (Game|SpawnActorfromClass "/Game/KrakJam/BP_Character.BP_Character_C" (Math|Transform|MakeTransform (+ (Variables|Default|GetLastTeleportDestination) "0, 0,200.000000") (Variables|Default|GetLastTeleportRotation) "1,1,1") "AdjustIfPossibleButAlwaysSpawn" 0 0))
  (Pawn|Possess (Game|GetPlayerController 0) _returnvalue)
  (bind _outactors (Actor|GetAllActorsOfClass "/Script/ApexDestruction.DestructibleActor"))
  (for _array_element _outactors
    (Actor|DestroyActor _array_element)))