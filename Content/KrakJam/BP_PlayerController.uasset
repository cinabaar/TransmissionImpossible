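; Player controller that adds a bullet time mechanic on FireSecondary and creates a BulletTimeTimer widget linked to itself.
; While held, Tick eases global time dilation down and drains the counter in undilated seconds until empty.
; Otherwise time eases back to normal, and a DoOnce-gated timer starts refilling the counter after a short delay.
; An older Timeline-based dilation approach remains in the graph but is never run.
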(event Custom|StartRefilling
  (Variables|Default|SetRefillOn true))

(event EventBeginPlay
  (bind _returnvalue (UserInterface|CreateWidget "/Game/KrakJam/BulletTimeTimer.BulletTimeTimer_C" self))
  (UserInterface|Viewport|AddtoViewport _returnvalue 0)
  (Variables|Default|SetBulletTimeCounter (Variables|Default|GetBulletTimeCounterMax))
  (Variables|/Game/KrakJam/BulletTimeTimer.BulletTimeTimer_C|SetController _returnvalue self))

(event EventTick
  (params (DeltaSeconds :type Float%20%28single-precision%29))
  (Utilities|FlowControl|Sequence
    (:then_0
      (if (Variables|Default|GetSlomoOn)
        (Variables|Default|SetRefillOn false)
        (Utilities|FlowControl|Sequence
          (:then_0
            (bind _output_get (Variables|Default|SetBulletTimeCounter (Math|Float|Max(Float) (- (Variables|Default|GetBulletTimeCounter) (/ DeltaSeconds (Class|GameplayStatics|GetGlobalTimeDilation))) 0.0)))
            (Utilities|Time|SetGlobalTimeDilation (Math|Interpolation|FInterptoConstant (Class|GameplayStatics|GetGlobalTimeDilation) 0.3 (Utilities|Time|GetWorldDeltaSeconds) 1.5))
            (if (== _output_get 0.0)
              (Variables|Default|SetSlomoOn false)))
          (:then_1
            (goto _label Reset)))
        (else
          (Utilities|FlowControl|Sequence
            (:then_0
              (Utilities|Time|SetGlobalTimeDilation (Math|Interpolation|FInterptoConstant (Class|GameplayStatics|GetGlobalTimeDilation) 1.0 (Utilities|Time|GetWorldDeltaSeconds) 1.0)))
            (:then_1
              (if (< (Variables|Default|GetBulletTimeCounter) (Variables|Default|GetBulletTimeCounterMax))
                (Utilities|FlowControl|DoOnce false :!label _label
                  (:Completed
                    (Utilities|Time|SetTimerbyEvent (delegate Custom|StartRefilling) 1.0)))))))))
    (:then_1
      (if (Variables|Default|GetRefillOn)
        (bind _output_get_2 (Variables|Default|SetBulletTimeCounter (Math|Float|Clamp(Float) (+ (Variables|Default|GetBulletTimeCounter) DeltaSeconds) 0.0 (Variables|Default|GetBulletTimeCounterMax))))
        (if (== _output_get_2 (Variables|Default|GetBulletTimeCounterMax))
          (Variables|Default|SetRefillOn false)
          (goto _label Reset))))))

(event Input|ActionEvents|InputActionFire
  (params (Key :type Key%20Structure)))

(event Input|ActionEvents|InputActionFireSecondary
  (params (Key :type Key%20Structure))
  (:Pressed
    (if (> (Variables|Default|GetBulletTimeCounter) 0.0)
      (Variables|Default|SetSlomoOn true)))
  (:Released
    (Variables|Default|SetSlomoOn false)))

(fn ConstructionScript)